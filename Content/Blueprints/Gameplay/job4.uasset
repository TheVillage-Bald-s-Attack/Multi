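; Job station actor for job slot 4 that the Citizen works at by interacting repeatedly.
; Box overlap toggles the prompt text and the NearToJob flag on GameplayPC, and leaving resets the current work progress.
; Each Interact call advances progress while JobCheck[4] is true; completion adds to TotalJobProgress and clears that flag.
; When the flag is false, interacting shows the NotWork indicator instead.
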(event OnComponentEndOverlap(Box)
  (params (OverlappedComponent :type Primitive%20Component%20Object%20Reference) (OtherActor :type Actor%20Object%20Reference) (OtherComp :type Primitive%20Component%20Object%20Reference) (OtherBodyIndex :type Integer))
  (if (== (Utilities|GetClass OtherActor) "/Game/Blueprints/Characters/Citizen.Citizen_C")
    (Rendering|SetVisibility (Variables|Default|GetTextRender) false false)
    (bind _asgameplay_pc (Utilities|Casting|CastToGameplayPC (Game|GetPlayerController 0)))
    (Variables|/Game/Blueprints/Gameplay/GameplayPC.GameplayPC_C|SetNearToJob _asgameplay_pc false)
    (Variables|/Game/Blueprints/Gameplay/GameplayPC.GameplayPC_C|SetWorkingJobProgress _asgameplay_pc 0.0)))

(event OnComponentBeginOverlap(Box)
  (params (OverlappedComponent :type Primitive%20Component%20Object%20Reference) (OtherActor :type Actor%20Object%20Reference) (OtherComp :type Primitive%20Component%20Object%20Reference) (OtherBodyIndex :type Integer) (bFromSweep :type Boolean) (SweepResult :type Hit%20Result%20Structure%20%28by%20ref%29))
  (if (== (Utilities|GetClass OtherActor) "/Game/Blueprints/Characters/Citizen.Citizen_C")
    (Rendering|SetVisibility (Variables|Default|GetTextRender) true false)
    (bind _asgameplay_pc (Utilities|Casting|CastToGameplayPC (Game|GetPlayerController 0)))
    (Variables|/Game/Blueprints/Gameplay/GameplayPC.GameplayPC_C|SetNearToJob _asgameplay_pc true)))

(event Custom|Working
  (Rendering|SetVisibility (Variables|Default|GetTextRender) false false)
  (bind _asgameplay_pc (Utilities|Casting|CastToGameplayPC (Game|GetPlayerController 0)))
  (if (Utilities|Array|Get(acopy) (Variables|/Game/Blueprints/Gameplay/GameplayPC.GameplayPC_C|GetJobCheck _asgameplay_pc) 4)
    (if (< (Variables|/Game/Blueprints/Gameplay/GameplayPC.GameplayPC_C|GetWorkingJobProgress _asgameplay_pc) 1.0)
      (bind _output_get (Variables|/Game/Blueprints/Gameplay/GameplayPC.GameplayPC_C|SetWorkingJobProgress _asgameplay_pc (+ (Variables|/Game/Blueprints/Gameplay/GameplayPC.GameplayPC_C|GetWorkingJobProgress _asgameplay_pc) 0.1)))
      (if (>= _output_get 1.0)
        (Variables|/Game/Blueprints/Gameplay/GameplayPC.GameplayPC_C|SetTotalJobProgress _asgameplay_pc (+ (Variables|/Game/Blueprints/Gameplay/GameplayPC.GameplayPC_C|GetTotalJobProgress _asgameplay_pc) 0.2))
        (Utilities|Array|SetArrayElem (Variables|/Game/Blueprints/Gameplay/GameplayPC.GameplayPC_C|GetJobCheck _asgameplay_pc) 4 false)))
    (else
      (Rendering|SetVisibility (Variables|Default|GetNotWork) true false))))

(fn ConstructionScript)

(fn Interact
  (CallFunction|Working)
  (return false))