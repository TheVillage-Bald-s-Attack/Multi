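; Gameplay player controller that handles spawning, chat and the vote screen for each player.
; On BeginPlay the local controller loads saved player settings, creates the vote widget and passes the settings to the server, where GameplayGM respawns the character before chat setup.
; Chat messages fan out through the GameMode's controller list to update each player's chat widget.
; T toggles the mouse cursor and V toggles the vote screen.
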(event Custom|PassCharacterInfoToServer
  (params (PlayerSettingsInfo :type Player%20Info%20Structure))
  ;[1 1 1] 캐릭터 정보를 서버에 보내주고 / 플레이어가 선택한 캐릭터를 스폰함
  (Variables|Default|SetPlayerSettings PlayerSettingsInfo)
  (bind _asgameplay_gm (Utilities|Casting|CastToGameplayGM (Game|GetGameMode)))
  (Default|RespawnPlayer _asgameplay_gm self (.IsBald (Utilities|Struct|BreakPlayerInfo (Variables|Default|GetPlayerSettings))))
  (CallFunction|SetupChatWindow))

(event Custom|SetupChatWindow
  ;[1 1 1] 게임 플레이 내의 채팅창을 만들고 뷰포트에 추가
  (bind _returnvalue (UserInterface|CreateWidget "/Game/UI/AllLevels/GameplayChat.GameplayChat_C"))
  (bind _output_get (Variables|Default|SetGameplayChatWB _returnvalue))
  (UserInterface|Viewport|AddtoViewport _output_get 0))

(event Custom|GetChatMessage
  (params (TextToSend :type Text))
  ;[1 1 1] 채팅입력처리/ 클라이언트에게 채팅정보 업데이트 통보
  (Variables|Default|SetSenderText TextToSend)
  (Variables|Default|SetSenderName (.MyPlayerName (Utilities|Struct|BreakPlayerInfo (Variables|Default|GetPlayerSettings))))
  (bind _asgameplay_gm (Utilities|Casting|CastToGameplayGM (Game|GetGameMode)))
  (for _array_element (Variables|/Game/Blueprints/Gameplay/GameplayGM.GameplayGM_C|GetAllPlayerControllers _asgameplay_gm)
    (bind _asgameplay_pc (Utilities|Casting|CastToGameplayPC _array_element))
    (CallFunction|UpdateChat _asgameplay_pc (Variables|Default|GetSenderName) (Variables|Default|GetSenderText))))

(event Custom|SetupVoteUI
  (bind _returnvalue (UserInterface|CreateWidget "/Game/UI/InGame/VoteUI.VoteUI_C"))
  (Variables|Default|SetVoteUI _returnvalue))

(event Custom|AddPlayerInfo
  (params (ConnectedPlayersInfo :type Array%20of%20Player%20Info%20Structures))
  (Variables|Default|SetAllConnectedPlayers ConnectedPlayersInfo))

(event Custom|ShowVoteScreen
  (bind _voteui (Variables|Default|GetVoteUI))
  (if (UserInterface|Viewport|IsinViewport _voteui)
    (if (Widget|IsVisible _voteui)
      (Widget|SetVisibility _voteui "Hidden")
      (else
        (Widget|SetVisibility _voteui "Visible")))
    (else
      (UserInterface|Viewport|AddtoViewport _voteui 0))))

(event Custom|UpdateChat
  (params (SenderName :type Text) (SenderText :type Text))
  ;[1 1 1] 클라이언트의 채팅창을 업데이트
  (Default|UpdateChatWindow (Variables|/Game/UI/AllLevels/GameplayChat.GameplayChat_C|GetGameplayChat (Variables|Default|GetGameplayChatWB)) SenderName SenderText))

(event EventBeginPlay
  ;[1 1 1] 플레이어 정보를 불러와 서버상 플레이어 컨트롤러에 넘겨줌
  (if (Pawn|IsLocalController)
    (Viewport|RemoveAllWidgets)
    (CallFunction|LoadGame)
    (CallFunction|SetupVoteUI)
    (CallFunction|PassCharacterInfotoServer (Variables|Default|GetPlayerSettings))
    (Development|PrintText (Utilities|Text|FormatText "{name} now here!" (.MyPlayerName (Utilities|Struct|BreakPlayerInfo (Variables|Default|GetPlayerSettings)))))))

(event Input|KeyboardEvents|V
  (params (Key :type Key%20Structure :default "None"))
  (:Pressed
    (CallFunction|ShowVoteScreen)))

(event Input|KeyboardEvents|T
  (params (Key :type Key%20Structure :default "None"))
  ;[1 1 1] T로 마우스 커서 컨트롤
  (:Pressed
    (Utilities|FlowControl|FlipFlop
      (:A
        (Variables|Default|SetbShowMouseCursor true))
      (:B
        (Variables|Default|SetbShowMouseCursor false)))))

(fn ConstructionScript)

(fn LoadGame
  (bind _returnvalue (SaveGame|LoadGamefromSlot (Variables|Default|GetPlayerSettingsSave)))
  (bind _asplayer_save_game (Utilities|Casting|CastToPlayerSaveGame _returnvalue))
  (Variables|Default|SetPlayerSettings (Variables|/Game/Blueprints/AllLevels/PlayerSaveGame.PlayerSaveGame_C|GetS_PlayerInfo _asplayer_save_game)))