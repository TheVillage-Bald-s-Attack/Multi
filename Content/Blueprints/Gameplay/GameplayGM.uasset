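; Game mode for a multiplayer Bald-versus-Citizen game that spawns players, assigns the bald role and runs a scalp-heat Fever meter.
; Tracks controllers, spawns pawns at random PlayerStarts, shares player settings with everyone, and handles session teardown and vote-list refresh.
; A delayed timer randomly flags a non-zero-index player as bald and shows UI.
; Fever climbs on a looping timer and drains while a sunward trace from player 0 detects shade.
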(event Custom|RespawnPlayer
  (params (PlayerController :type Player%20Controller%20Object%20Reference) (IsBald :type Boolean))
  ;[1 1 1] 캐릭터를 게임 플레이 컨트롤러에서 받아서 스폰시켜줌
  (bind _outactors (Actor|GetAllActorsOfClass "/Script/Engine.PlayerStart"))
  (Variables|Default|SetPlayerController PlayerController)
  (Variables|GameInfo|SetSpawnPoints _outactors)
  (if IsBald
    (bind _returnvalue (Game|SpawnActorfromClass "/Game/Blueprints/Characters/Bald.Bald_C" (Transformation|GetActorTransform (Utilities|Array|Get(acopy) (Variables|GameInfo|GetSpawnPoints) (Math|Random|RandomIntegerinRange 0 (- (Utilities|Array|Length (Variables|GameInfo|GetSpawnPoints)) 1)))) "Undefined" 0 0))
    (Pawn|Possess PlayerController _returnvalue)
    (Variables|Default|SetBaldCount (+ (Variables|Default|GetBaldCount) 1))
    (else
      (bind _returnvalue_2 (Game|SpawnActorfromClass "/Game/Blueprints/Characters/Citizen.Citizen_C" (Transformation|GetActorTransform (Utilities|Array|Get(acopy) (Variables|GameInfo|GetSpawnPoints) (Math|Random|RandomIntegerinRange 0 (- (Utilities|Array|Length (Variables|GameInfo|GetSpawnPoints)) 1)))) "Undefined" 0 0))
      (Pawn|Possess PlayerController _returnvalue_2)
      (Variables|Default|SetCitizenCount (+ (Variables|Default|GetCitizenCount) 1))))
  (Variables|Default|SetTotalPlayerCount (+ (Variables|Default|GetTotalPlayerCount) 1))
  (CallFunction|EveryoneUpdate))

(event Custom|EveryoneUpdate
  (bind _allplayercontrollers (Variables|GameInfo|GetAllPlayerControllers))
  ;[1 1 1] 호출시 접속자들에게 게임모드 정보 업데이트
  (if (> (Variables|Default|GetTotalPlayerCount) 0)
    (Utilities|Array|Clear (Variables|GameInfo|GetConnectedPlayers))
    (for _array_element _allplayercontrollers
      (bind _asgameplay_pc (Utilities|Casting|CastToGameplayPC _array_element))
      (Utilities|Array|Add (Variables|GameInfo|GetConnectedPlayers) (Variables|/Game/Blueprints/Gameplay/GameplayPC.GameplayPC_C|GetPlayerSettings _asgameplay_pc)))
    (for _array_element_2 _allplayercontrollers
      (bind _asgameplay_pc_2 (Utilities|Casting|CastToGameplayPC _array_element_2))
      (Default|AddPlayerInfo _asgameplay_pc_2 (Variables|GameInfo|GetConnectedPlayers)))))

(event Custom|AddFeverToBald
  ;[1 1 1] 대머리일 경우, 그늘에 있지 않을 때 두피열 추가
  (if (<= (+ (Variables|Default|GetFever) (/ 0.01 5e+01)) 1.0)
    (Variables|Default|SetFever (+ (Variables|Default|GetFever) (/ 0.01 5e+01)))))

(event Custom|AddToVoteList
  ;[1 1 1] 게임 설정창이 열려있어도 플레이어를 추방 목록에 추가함
  (bind _asgameplay_pc (Utilities|Casting|CastToGameplayPC (Game|GetPlayerController 0)))
  (Default|FillPlayersWindow (Variables|/Game/Blueprints/Gameplay/GameplayPC.GameplayPC_C|GetVoteUI _asgameplay_pc)))

(event EventPostLogin
  (params (NewPlayer :type Player%20Controller%20Object%20Reference))
  (Utilities|Array|Add (Variables|GameInfo|GetAllPlayerControllers) NewPlayer))

(event EventOnLogout
  (params (ExitingController :type Controller%20Object%20Reference))
  ;[1 1 1] 로그아웃시 세션 파기 호출
  (bind _asgameplay_pc (Utilities|Casting|CastToGameplayPC ExitingController))
  (Default|DestroySessionCaller (.AsGame%20Info%20Instance (Utilities|Casting|CastToGameInfoInstance (Game|GetGameInstance))) _asgameplay_pc))

(event EventBeginPlay
  ;[1 1 1] BeginPlay
  (CallFunction|SetSunlight)
  (Utilities|Time|SetTimerbyFunctionName 0 "AssignPlayers" 5.0)
  (Utilities|FlowControl|Delay 2.5)
  (Utilities|Time|SetTimerbyEvent (delegate Custom|AddFeverToBald) 0.01 true))

(event EventOnSwapPlayerControllers
  (params (OldPC :type Player%20Controller%20Object%20Reference) (NewPC :type Player%20Controller%20Object%20Reference))
  ;[1 1 1] 서버 접속자의 플레이어 컨트롤러 추적
  (Utilities|Array|Add (Variables|GameInfo|GetAllPlayerControllers) NewPC))

(event EventTick
  (params (DeltaSeconds :type Float%20%28single-precision%29))
  ;[1 1 1] 그늘에 있을 때 두피열 줄이ㅏ기
  (CallFunction|CheckIsonShadw)
  (if (not (Variables|PlayerInfo|GetIsVisible))
    (if (>= (- (Variables|Default|GetFever) (/ DeltaSeconds 15.0)) 0.0)
      (Variables|Default|SetFever (- (Variables|Default|GetFever) (/ DeltaSeconds 15.0))))))

(fn ConstructionScript
  (|CallParentFunction))

(fn SetSunlight
  (bind _outactors (Actor|GetAllActorsOfClass "/Script/Engine.DirectionalLight"))
  (Variables|Default|SetSun (Utilities|Array|Get(acopy) _outactors)))

(fn CheckIsonShadw
  (bind _returnvalue (Game|Player|GetPlayerPawn 0))
  (bind _returnvalue_2 (Transformation|GetActorLocation _returnvalue))
  (bind _returnvalue_3 (Collision|LineTraceByChannel _returnvalue_2 (+ _returnvalue_2 (* (Transformation|GetActorForwardVector (Variables|Default|GetSun)) -100000)) "TraceTypeQuery1" false 0 "None"))
  (if _returnvalue_3
    (Variables|PlayerInfo|SetIsVisible false)
    (Development|PrintText "On Shadow" true true "(R=0.000000,G=0.660000,B=1.000000,A=1.000000)" 0.0)
    (else
      (Variables|PlayerInfo|SetIsVisible true)
      (Development|PrintText "Not On Shadow" true true "(R=0.000000,G=0.660000,B=1.000000,A=1.000000)" 0.0))))

(fn AssignPlayers
  (bind _totalplayercount (Variables|Default|GetTotalPlayerCount))
  (Development|PrintString (Utilities|String|ToString(Integer) _totalplayercount))
  (bind _output_get (Variables|Default|SetBaldUserIndex (Math|Random|RandomIntegerinRange 1 (- _totalplayercount 1))))
  (Development|PrintText (Utilities|Text|ToText(Integer) _output_get))
  (bind _asgameplay_pc (Utilities|Casting|CastToGameplayPC (Game|GetPlayerController _output_get)))
  (bind _structout (Utilities|Struct|SetmembersinPlayerInfo (Variables|/Game/Blueprints/Gameplay/GameplayPC.GameplayPC_C|GetPlayerSettings _asgameplay_pc) true))
  (Variables|PlayerInfo|SetBaldPlayerSettings _structout)
  (Variables|/Game/Blueprints/Gameplay/GameplayPC.GameplayPC_C|SetPlayerSettings _asgameplay_pc _structout)
  (bind _returnvalue (UserInterface|CreateWidget "/Game/UI/InGame/PrintIsBald.PrintIsBald_C" 0 true))
  (UserInterface|Viewport|AddtoViewport _returnvalue 0)
  (bind _returnvalue_2 (UserInterface|CreateWidget "/Game/UI/InGame/FeverUI.FeverUI_C"))
  (UserInterface|Viewport|AddtoViewport _returnvalue_2 0))