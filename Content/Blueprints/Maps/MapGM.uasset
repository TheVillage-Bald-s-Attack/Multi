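; Map game mode for a game with Bald and Citizen roles, handling sun exposure, role display and voting UI.
; While IsBald is set, Tick line-traces from player 0 toward the first directional light and gradually lowers the Bald pawn's Fever in shadow, printing debug status.
; CheckIsBaldOrCitizen spawns a role widget per LobbyPC connected player; StartVote opens VoteUI.
; SetPlayersType, Vote and EndVote are empty stubs.
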(event Custom|StartVote
  (bind _returnvalue (UserInterface|CreateWidget "/Game/UI/InGame/VoteUI.VoteUI_C"))
  (UserInterface|Viewport|AddtoViewport _returnvalue 0))

(event EventBeginPlay
  (CallFunction|SetSunlight))

(event EventTick
  (params (DeltaSeconds :type Float%20%28single-precision%29))
  ;[1 1 1] Tick 이벤트 - 대머리가 그늘에 있을 경우 두피열 감소 기능
  (if (Variables|Default|GetIsBald)
    (CallFunction|CheckSunlight)
    (if (Variables|Default|GetIsVisible)
      (Development|PrintText "Not On Shadow" true false "(R=0.000000,G=0.660000,B=1.000000,A=1.000000)" 0.0)
      (else
        (Development|PrintText "On Shadow" true false "(R=0.000000,G=0.660000,B=1.000000,A=1.000000)" 0.0)
        (bind _asbald (Utilities|Casting|CastToBald (Game|Player|GetPlayerPawn 0)))
        (if (>= (- (Variables|/Game/Blueprints/Characters/Bald.Bald_C|GetFever _asbald) (/ DeltaSeconds 15.0)) 0.0)
          (Variables|/Game/Blueprints/Characters/Bald.Bald_C|SetFever _asbald (- (Variables|/Game/Blueprints/Characters/Bald.Bald_C|GetFever _asbald) (/ DeltaSeconds 15.0))))))))

(fn ConstructionScript
  (|CallParentFunction))

(fn CheckSunlight
  (bind _returnvalue (Game|Player|GetPlayerPawn 0))
  (bind _returnvalue_2 (Transformation|GetActorLocation _returnvalue))
  (bind _returnvalue_3 (Collision|LineTraceByChannel _returnvalue_2 (+ _returnvalue_2 (* (Transformation|GetActorForwardVector (Variables|Default|GetSun)) -100000)) "TraceTypeQuery1" false 0 "None"))
  (if _returnvalue_3
    (Variables|Default|SetIsVisible false)
    (else
      (Variables|Default|SetIsVisible true))))

(fn CheckIsBaldorCitizen
  (bind _aslobby_pc (Utilities|Casting|CastToLobbyPC (Game|GetPlayerController 0))
    (:then
      (for _array_element (Variables|/Game/Blueprints/Lobby/LobbyPC.LobbyPC_C|GetAllConnectedPlayers _aslobby_pc)
        (if (.IsBald (Utilities|Struct|BreakPlayerInfo _array_element))
          (bind _returnvalue (UserInterface|CreateWidget "/Game/UI/InGame/PrintIsBald.PrintIsBald_C" 0 (.IsBald (Utilities|Struct|BreakPlayerInfo _array_element))))
          (else
            (bind _returnvalue_2 (UserInterface|CreateWidget "/Game/UI/InGame/PrintIsBald.PrintIsBald_C" 0 (.IsBald (Utilities|Struct|BreakPlayerInfo _array_element))))))
        (UserInterface|Viewport|AddtoViewport _returnvalue 0)))
    (:CastFailed
      (Development|PrintText "Cast failed"))))

(fn SetSunlight
  (bind _outactors (Actor|GetAllActorsOfClass "/Script/Engine.DirectionalLight"))
  (Variables|Default|SetSun (Utilities|Array|Get(acopy) _outactors)))

(fn SetPlayersType
  (params (PlayerInfo :type Player%20Info%20Structure)))

(fn EndVote)

(fn Vote)