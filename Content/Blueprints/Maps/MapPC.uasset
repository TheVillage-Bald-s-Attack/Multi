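; MapPC, by its name the map's player controller, shows on screen whether each connected player is bald or a citizen.
; On BeginPlay it casts player controller 0 to LobbyPC and loops over its AllConnectedPlayers list.
; Each entry gets a PrintIsBald widget carrying its IsBald flag, added to the viewport; both branches create the same widget class.
; A failed cast only prints a message.
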(event EventBeginPlay
  (CallFunction|CheckIsBaldorCitizen))

(fn ConstructionScript)

(fn CheckIsBaldorCitizen
  (bind _aslobby_pc (Utilities|Casting|CastToLobbyPC (Game|GetPlayerController 0))
    (:then
      (for _array_element (Variables|/Game/Blueprints/Lobby/LobbyPC.LobbyPC_C|GetAllConnectedPlayers _aslobby_pc)
        (if (.IsBald (Utilities|Struct|BreakPlayerInfo _array_element))
          (bind _returnvalue (UserInterface|CreateWidget "/Game/UI/InGame/PrintIsBald.PrintIsBald_C" 0 (.IsBald (Utilities|Struct|BreakPlayerInfo _array_element))))
          (else
            (bind _returnvalue_2 (UserInterface|CreateWidget "/Game/UI/InGame/PrintIsBald.PrintIsBald_C" 0 (.IsBald (Utilities|Struct|BreakPlayerInfo _array_element))))))
        (UserInterface|Viewport|AddtoViewport _returnvalue 0)))
    (:CastFailed
      (Development|PrintText "Cast failed"))))