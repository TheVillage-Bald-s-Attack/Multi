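; Bald character Blueprint that tracks a Fever value building up over time during play.
; On BeginPlay it creates a FeverUI widget and adds it to the viewport.
; Each Tick raises Fever in proportion to delta time, filling the full range in about fifty seconds and skipping any step that would exceed one.
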(event EventBeginPlay
  (bind _returnvalue (UserInterface|CreateWidget "/Game/UI/InGame/FeverUI.FeverUI_C"))
  (UserInterface|Viewport|AddtoViewport _returnvalue 0))

(event EventTick
  (params (DeltaSeconds :type Float%20%28single-precision%29))
  (if (<= (+ (/ DeltaSeconds 5e+01) (Variables|Default|Getfever)) 1.0)
    (Variables|Default|Setfever (+ (/ DeltaSeconds 5e+01) (Variables|Default|Getfever)))))

(fn ConstructionScript
  (|CallParentFunction))